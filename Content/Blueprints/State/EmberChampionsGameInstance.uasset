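; Game instance for Ember Champions that holds the volume setting and the currently selected champion card.
; ChangeVolume only stores the new value in a variable.
; SetSelected enforces single selection: it toggles off the previous card, then stores and toggles on the new one, or clears the selection when the same card is passed again.
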(event `ChangeVolume`
  (params (NewVolume :type "Float (double-precision)"))
  ; Save Volume Setting
  (set `self.Volume` NewVolume))

(event `SetSelected`
  (params (SelectedWidget :type "/Game/UI/CharacterCardWidget Object Reference"))
  (bind _selectedcard (`self.SelectedCard`))
  ; Set Selected Champion
  (if (`KismetSystemLibrary.IsValid` _selectedcard)
    (`/Game/UI/CharacterCardWidget.ToggleSelected` _selectedcard))
  (bind _output_get (set `self.SelectedCard` (select `bool` (== SelectedWidget _selectedcard) :`false` SelectedWidget)))
  (if (`KismetSystemLibrary.IsValid` _output_get)
    (`/Game/UI/CharacterCardWidget.ToggleSelected` _output_get)))