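; GameStateBP is a state Blueprint that spawns champions and tracks them as the player's squad members.
; SpawnSelected caches the player character as the Squad, reads the starting member class from EmberChampionsGameInstance and passes it to AddChampion.
; AddChampion spawns that class at a fixed elevated transform, appends it to SquadMembers and hands the whole array to the Squad.
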(event `Spawn Selected`
  ; Spawns the selected champion
  (bind _assquad (cast `/Game/Blueprints/Squad` (`GameplayStatics.GetPlayerCharacter` 0)))
  (set `self.SquadRef` _assquad)
  (bind _asember_champions_game_instance (cast `/Game/Blueprints/State/EmberChampionsGameInstance` (`GameplayStatics.GetGameInstance`)))
  (`self.Add Champion` (`/Game/Blueprints/State/EmberChampionsGameInstance.StartingMember` _asember_champions_game_instance)))

(event `Add Champion`
  (params (Champion :type "/Game/Blueprints/Entities/Champions/ChampionBP Class Reference"))
  (bind _squadmembers (`self.SquadMembers`))
  ; Add a specified champion to the squad
  (bind _returnvalue (`|SpawnActorFromClass` Champion (`KismetMathLibrary.MakeTransform` (0.0 0.0 1000.0)) "Undefined" "MultiplyWithRoot" null null))
  (`KismetArrayLibrary.Array_Add` _squadmembers _returnvalue)
  (`/Game/Blueprints/Squad.Add Champions` (`self.SquadRef`) _squadmembers))

(fn `UserConstructionScript`)