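; EnvironmentalHazards is a spawner actor that continuously drops meteors and fire hazards across a wide area around itself.
; On BeginPlay it starts two looping timers, with meteors spawning twice as often as fires.
; Each spawn picks a random XY point in a rectangle centred on the actor at a fixed world height.
; Meteors appear high up with random rotation, while scaled-up fires appear unrotated near ground level.
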(event `SpawnMeteors`
  (bind _x (.x (`self.K2_GetActorLocation`)))
  (bind _y (.y (`self.K2_GetActorLocation`)))
  (`|SpawnActorFromClass` "/Game/Blueprints/MeteorBP.MeteorBP_C" (`KismetMathLibrary.MakeTransform` (`KismetMathLibrary.MakeVector` (`KismetMathLibrary.RandomFloatInRange` (- _x 6000.0) (+ _x 6000.0)) (`KismetMathLibrary.RandomFloatInRange` (- _y 3500.0) (+ _y 3500.0)) 1250.0) (`KismetMathLibrary.RandomRotator` false)) "Undefined" "MultiplyWithRoot" null null))

(event `self.ReceiveTick`
  (params (DeltaSeconds :type "Float (single-precision)")))

(event `self.ReceiveBeginPlay`
  (`|ExecutionSequence`
    (:`then_0`
      (`KismetSystemLibrary.K2_SetTimerDelegate` (delegate `SpawnMeteors`) 0.5 true))
    (:`then_1`
      (`KismetSystemLibrary.K2_SetTimerDelegate` (delegate `SpawnFires`) 1.0 true))))

(event `SpawnFires`
  (bind _x (.x (`self.K2_GetActorLocation`)))
  (bind _y (.y (`self.K2_GetActorLocation`)))
  (`|SpawnActorFromClass` "/Game/Blueprints/FireHazardBP.FireHazardBP_C" (`KismetMathLibrary.MakeTransform` (`KismetMathLibrary.MakeVector` (`KismetMathLibrary.RandomFloatInRange` (- _x 6000.0) (+ _x 6000.0)) (`KismetMathLibrary.RandomFloatInRange` (- _y 3500.0) (+ _y 3500.0)) 100.0) (struct) (3.0 3.0 3.0)) "Undefined" "MultiplyWithRoot" null null))

(fn `UserConstructionScript`)