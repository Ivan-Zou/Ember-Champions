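; MeteorBP is a meteor actor that tumbles and explodes when it hits certain actors.
; Tick adds a fixed local rotation to MeteorCollider each frame, not scaled by delta time.
; On component hit, a Sequence of casts checks for dragon, fire golem, fire dog, stone, jail or blocking volume.
; Any match shares one path that destroys the meteor, spawns ExplosionBP at its location and plays a quiet explosion sound.
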(event `self.ReceiveTick`
  (params (DeltaSeconds :type "Float (single-precision)"))
  (`SceneComponent.K2_AddLocalRotation` (`self.MeteorCollider`) (struct :`Pitch` 5.0 :`Yaw` 5.0 :`Roll` 5.0) false false))

(event `self.MeteorCollider.OnComponentHit`
  (params (HitComponent :type "PrimitiveComponent Object Reference") (OtherActor :type "Actor Object Reference") (OtherComp :type "PrimitiveComponent Object Reference") (NormalImpulse :type "Vector Structure") (Hit :type "HitResult Structure (by ref)"))
  (bind _returnvalue (`self.K2_GetActorLocation`))
  (`|ExecutionSequence`
    (:`then_0`
      (cast `/Game/Blueprints/DragonBP` OtherActor))
    (:`then_1`
      (cast `/Game/Blueprints/FireGolemBP` OtherActor))
    (:`then_2`
      (cast `/Game/Blueprints/FireDogBP` OtherActor))
    (:`then_3`
      (cast `/Game/Blueprints/StoneBP` OtherActor))
    (:`then_4`
      (cast `/Game/Blueprints/JailBP` OtherActor))
    (:`then_5`
      (cast `BlockingVolume` OtherActor)))
  (`self.K2_DestroyActor`)
  (`|SpawnActorFromClass` "/Game/Particles/ExplosionBP.ExplosionBP_C" (`KismetMathLibrary.MakeTransform` _returnvalue) "Undefined" "MultiplyWithRoot" null null)
  (`GameplayStatics.PlaySoundAtLocation` "/Game/StarterContent/Audio/Explosion01.Explosion01" _returnvalue (struct) 0.05 1.0 0.0 null null null null))

(fn `UserConstructionScript`)