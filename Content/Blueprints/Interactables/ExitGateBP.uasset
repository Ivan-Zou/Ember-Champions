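; Exit gate interactable that ends the level with a result screen once the squad has enough embers.
; HandleInteraction compares the squad's ember count to the requirement, showing a brief alert if it falls short.
; Otherwise it toggles the HUD, pauses the game and initializes the result screen.
; Tick separately opens the main menu once game time passes a positive Timeout, which is not set in these graphs.
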(event `self.ReceiveTick`
  (params (DeltaSeconds :type "Float (single-precision)"))
  (bind _timeout (`self.Timeout`))
  (if (and (> _timeout 0.0) (< _timeout (`KismetSystemLibrary.GetGameTimeInSeconds`)))
    (`GameplayStatics.OpenLevelBySoftObjectPtr` "/Game/Levels/MainMenu.MainMenu")))

(fn `HandleInteraction`
  (if (< (`/Game/Blueprints/Squad.EmberCount` (`self.SquadRef`)) (`self.EmberRequirement`))
    (bind _returnvalue (`|CreateWidget` "/Game/UI/AlertWidget.AlertWidget_C"))
    (`UserWidget.AddToViewport` _returnvalue 0)
    (`/Game/UI/AlertWidget.Start Alert` _returnvalue (`KismetStringLibrary.Concat_StrStr` "You need " (`KismetStringLibrary.Conv_IntToString` (`self.EmberRequirement`)) " embers to EXIT!") 0.75)
    (else
      (`/Game/Blueprints/Squad.Toggle HUD` (`self.SquadRef`))
      (bind _returnvalue_2 (`|CreateWidget` "/Game/UI/ResultScreenWidget.ResultScreenWidget_C"))
      (`UserWidget.AddToViewport` _returnvalue_2 0)
      (`GameplayStatics.SetGamePaused` true)
      (`/Game/UI/ResultScreenWidget.Initialize` _returnvalue_2 true))))

(fn `UserConstructionScript`)