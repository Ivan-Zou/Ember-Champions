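; Chest interactable that spends one of the squad's keys to grant random loot, then destroys itself.
; HandleInteraction checks the squad's key count, calling GetRandomItem once per entry of a three-element loop, or showing a brief missing-key alert widget when none remain.
; GetRandomItem uses two nested random rolls to add an ember, upgrade point or potion, so the commented 50/40 split applies only after the 10% ember roll fails.
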(fn `GetRandomItem`
  (bind _returnvalue (`KismetMathLibrary.RandomFloatInRange` 0.0 1000.0))
  (if (< _returnvalue 100.0)
    (`self.Add Item` 0)
    (elif (< _returnvalue 600.0)
      (`self.Add Item` 2)
      (else
        (`self.Add Item` 3)))))

(fn `HandleInteraction`
  (bind _keycount (`/Game/Blueprints/Squad.KeyCount` (`self.SquadRef`)))
  (if (> _keycount 0)
    (bind _result (`/Engine/EditorBlueprintResources/StandardMacros.DecrementInt` _keycount) ; 10% of ember, 50% upgrade point, 40% potions
      (:`  `
        (for _ (`|MakeArray` _result 0 0)
          (`self.GetRandomItem`))
        (`self.K2_DestroyActor`)))
    (else
      (bind _returnvalue (`|CreateWidget` "/Game/UI/AlertWidget.AlertWidget_C"))
      (`UserWidget.AddToViewport` _returnvalue 0)
      (`/Game/UI/AlertWidget.Start Alert` _returnvalue "You are missing a key!" 0.75))))

(fn `UserConstructionScript`)