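; StoneBP is an interactable stone that breaks when used and occasionally drops an item.
; HandleInteraction makes a 5% drop roll, then nested rolls pick item 0, 1 or 2, commented as ancient ember, potion and key.
; Each roll is fresh, so the split is 10/63/27 rather than the commented 10/60/30.
; The stone always destroys itself and plays a collapse sound at its location.
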(fn `HandleInteraction`
  (bind _returnvalue (`KismetMathLibrary.RandomFloatInRange` 0.0 1000.0))
  (if (< (`KismetMathLibrary.RandomFloatInRange` 0.0 1000.0) 50.0)
    (if (< _returnvalue 100.0)
      (`self.Add Item` 0)
      (elif (< _returnvalue 700.0)
        (`self.Add Item` 1)
        (else
          (`self.Add Item` 2)))))
  (`self.K2_DestroyActor`)
  (`GameplayStatics.PlaySoundAtLocation` "/Game/StarterContent/Audio/Collapse01.Collapse01" (`self.K2_GetActorLocation`) (struct) 0.05 1.0 0.0 null null null null))

(fn `UserConstructionScript`)