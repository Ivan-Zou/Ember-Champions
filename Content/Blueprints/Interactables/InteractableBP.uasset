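; Base interactable actor that registers itself in the on-screen interaction list while a Squad overlaps its collider.
; BeginPlay grabs the first InteractListWidget; overlap begin caches the Squad and adds an entry with its InteractText, and overlap end removes it.
; HandleInteraction is an empty stub, and AddItem increments the cached Squad's ember, key, potion or upgrade count by item index.
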(event `self.ReceiveBeginPlay`
  (bind _foundwidgets (`WidgetBlueprintLibrary.GetAllWidgetsOfClass` "/Game/UI/InteractListWidget.InteractListWidget_C"))
  (set `self.InteractionListWidget` (`|GetArrayItem` _foundwidgets)))

(event `self.InteractionCollider.OnComponentBeginOverlap`
  (params (OverlappedComponent :type "PrimitiveComponent Object Reference") (OtherActor :type "Actor Object Reference") (OtherComp :type "PrimitiveComponent Object Reference") (OtherBodyIndex :type Integer) (bFromSweep :type Boolean) (SweepResult :type "HitResult Structure (by ref)"))
  (bind _assquad (cast `/Game/Blueprints/Squad` OtherActor))
  (set `self.SquadRef` _assquad)
  (`/Game/UI/InteractListWidget.Add Interaction` (`self.InteractionListWidget`) (`self.InteractText`) self))

(event `self.InteractionCollider.OnComponentEndOverlap`
  (params (OverlappedComponent :type "PrimitiveComponent Object Reference") (OtherActor :type "Actor Object Reference") (OtherComp :type "PrimitiveComponent Object Reference") (OtherBodyIndex :type Integer))
  (cast `/Game/Blueprints/Squad` OtherActor)
  (`/Game/UI/InteractListWidget.Remove Interaction` (`self.InteractionListWidget`) self))

(fn `Add Item`
  (params (ItemIndex :type Integer))
  (bind _squadref (`self.SquadRef`))
  (if (== ItemIndex 0)
    (`/Engine/EditorBlueprintResources/StandardMacros.IncrementInt` (`/Game/Blueprints/Squad.EmberCount` (`self.SquadRef`)))
    (elif (== ItemIndex 1)
      (`/Engine/EditorBlueprintResources/StandardMacros.IncrementInt` (`/Game/Blueprints/Squad.KeyCount` _squadref))
      (elif (== ItemIndex 2)
        (`/Engine/EditorBlueprintResources/StandardMacros.IncrementInt` (`/Game/Blueprints/Squad.PotionCount` _squadref))
        (else
          (`/Engine/EditorBlueprintResources/StandardMacros.IncrementInt` (`/Game/Blueprints/Squad.UpgradeCount` _squadref)))))))

(fn `HandleInteraction`)

(fn `UserConstructionScript`)