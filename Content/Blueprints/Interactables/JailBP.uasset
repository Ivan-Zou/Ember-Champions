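; Interactable jail that holds a trapped champion, which the squad can free by spending a key.
; SetTrapped stores the champion class, builds an "Unlock" prompt from its class defaults and shows it through a child actor component.
; On interaction, it uses one of the squad's keys, adds the champion through the game state and destroys itself.
; Without a key, it shows a brief alert widget saying a key is missing.
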(event `Set Trapped`
  (params (Trapped :type "/Game/Blueprints/Entities/Champions/ChampionBP Class Reference"))
  (bind _trappedchampion (`self.TrappedChampion`))
  (set `self.TrappedChampion` Trapped)
  (set `self.InteractText` (`KismetStringLibrary.Concat_StrStr` "Unlock " (defaults `Object` _trappedchampion)))
  (`ChildActorComponent.SetChildActorClass` (`self.ChildActor`) _trappedchampion))

(fn `HandleInteraction`
  (bind _keycount (`/Game/Blueprints/Squad.KeyCount` (`self.SquadRef`)))
  (if (> _keycount 0)
    (`/Engine/EditorBlueprintResources/StandardMacros.DecrementInt` _keycount
      (:`  `
        (`/Game/Blueprints/State/GameStateBP.Add Champion` (`/Game/Blueprints/Squad.GameStateObj` (`self.SquadRef`)) (`self.TrappedChampion`))
        (`self.K2_DestroyActor`)))
    (else
      (bind _returnvalue (`|CreateWidget` "/Game/UI/AlertWidget.AlertWidget_C"))
      (`UserWidget.AddToViewport` _returnvalue 0)
      (`/Game/UI/AlertWidget.Start Alert` _returnvalue "You are missing a key!" 0.75))))

(fn `UserConstructionScript`)