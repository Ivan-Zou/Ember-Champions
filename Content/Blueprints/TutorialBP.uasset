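; TutorialBP is an actor that periodically spawns meteor and fire hazards at randomized positions relative to itself.
; BeginPlay starts two looping timers, with meteors spawning more often than fires.
; Both spawn events offset along negative X from the actor's current location, randomize Y around it and use a fixed world height.
; Meteors get a random rotation, while fire hazards spawn unrotated, farther away and scaled up.
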(event `SpawnMeteors`
  (bind _y (.y (`self.K2_GetActorLocation`)))
  (`|SpawnActorFromClass` "/Game/Blueprints/MeteorBP.MeteorBP_C" (`KismetMathLibrary.MakeTransform` (`KismetMathLibrary.MakeVector` (+ (.x (`self.K2_GetActorLocation`)) -1250.0) (`KismetMathLibrary.RandomFloatInRange` (- _y 600.0) (+ _y 600.0)) 1250.0) (`KismetMathLibrary.RandomRotator` false)) "Undefined" "MultiplyWithRoot" null null))

(event `self.ReceiveBeginPlay`
  (`|ExecutionSequence`
    (:`then_0`
      (`KismetSystemLibrary.K2_SetTimerDelegate` (delegate `SpawnMeteors`) 3.0 true))
    (:`then_1`
      (`KismetSystemLibrary.K2_SetTimerDelegate` (delegate `SpawnFires`) 10.0 true))))

(event `SpawnFires`
  (bind _y (.y (`self.K2_GetActorLocation`)))
  (`|SpawnActorFromClass` "/Game/Blueprints/FireHazardBP.FireHazardBP_C" (`KismetMathLibrary.MakeTransform` (`KismetMathLibrary.MakeVector` (+ (.x (`self.K2_GetActorLocation`)) -2250.0) (`KismetMathLibrary.RandomFloatInRange` (- _y 700.0) (+ _y 700.0)) 100.0) (struct) (3.0 3.0 3.0)) "Undefined" "MultiplyWithRoot" null null))

(fn `UserConstructionScript`)