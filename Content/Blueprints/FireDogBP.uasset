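; Fire dog actor that starts a battle when the Squad comes within its detection radius.
; Each Tick, while the Squad has no active battle, it runs IsChampionNearby, then prints a debug message and calls InitiateBattle on the Squad with itself.
; Detection temporarily uses horizontal distance to the Squad actor; a disconnected per-member check awaits a populated Squad.
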(event `self.ReceiveTick`
  (params (DeltaSeconds :type "Float (single-precision)"))
  (bind _returnvalue (`GameplayStatics.GetActorOfClass` "/Game/Blueprints/Squad.Squad_C"))
  (if (not (`/Game/Blueprints/Squad.IsBattleActive` _returnvalue))
    (bind _returnval (`self.IsChampionNearby`))
    (if _returnval
      (`KismetSystemLibrary.PrintString` "DOG DETECTS SQUAD")
      (bind _returnvalue_2 (`GameplayStatics.GetActorOfClass` "/Game/Blueprints/Squad.Squad_C"))
      (`/Game/Blueprints/Squad.InitiateBattle` _returnvalue_2 self))))

(fn `IsChampionNearby`
  (returns (ReturnVal :type Boolean))
  ; (Temporary) This just uses the Squad Actor's Location
  (bind _returnvalue (`GameplayStatics.GetActorOfClass` "/Game/Blueprints/Squad.Squad_C"))
  (return (<= (`self.GetHorizontalDistanceTo` _returnvalue) (`self.detectionRadius`))))

(fn `UserConstructionScript`)