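; Dragon enemy Blueprint that starts a battle when the player's Squad comes within its detection radius.
; Each tick, while the Squad has no active battle, it tests horizontal distance to the Squad actor and, if in range, calls OnBattleInitiated on it with itself.
; The proximity check temporarily uses the Squad's own location; an unreachable per-member check awaits populated squad members.
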(event `self.ReceiveBeginPlay`
  (`parent.ReceiveBeginPlay`))

(event `self.ReceiveTick`
  (params (DeltaSeconds :type "Float (single-precision)"))
  (bind _returnvalue (`GameplayStatics.GetActorOfClass` "/Game/Blueprints/Squad.Squad_C"))
  (if (not (`/Game/Blueprints/Squad.IsBattleActive` _returnvalue))
    (bind _returnval (`self.IsChampionNearby`))
    (if _returnval
      (bind _returnvalue_2 (`GameplayStatics.GetActorOfClass` "/Game/Blueprints/Squad.Squad_C"))
      (`/Game/Blueprints/Squad.OnBattleInitiated` _returnvalue_2 self)
      (`KismetSystemLibrary.PrintString` "DRAGON DETECTS SQUAD"))))

(fn `IsChampionNearby`
  (returns (ReturnVal :type Boolean))
  ; (Temporary) This just uses the Squad Actor's Location
  (bind _returnvalue (`GameplayStatics.GetActorOfClass` "/Game/Blueprints/Squad.Squad_C"))
  (return (<= (`self.GetHorizontalDistanceTo` _returnvalue) (`self.detectionRadius`))))

(fn `UserConstructionScript`)