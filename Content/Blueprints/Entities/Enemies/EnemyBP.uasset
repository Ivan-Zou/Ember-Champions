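; Enemy entity Blueprint that starts a battle when a Squad enters its BattleCollider.
; Every Tick it polls the collider for overlapping Squad actors instead of relying on overlap events.
; For each Squad without an active battle, it calls OnBattleInitiated with itself as the argument and prints a debug message.
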(event `self.ReceiveTick`
  (params (DeltaSeconds :type "Float (single-precision)"))
  (for _array_element (`PrimitiveComponent.GetOverlappingActors` (`self.BattleCollider`) "/Game/Blueprints/Squad.Squad_C")
    (bind _assquad (cast `/Game/Blueprints/Squad` _array_element))
    (if (not (`/Game/Blueprints/Squad.IsBattleActive` _assquad))
      (`/Game/Blueprints/Squad.OnBattleInitiated` _assquad self)
      (`KismetSystemLibrary.PrintString` "Battle Initiated"))))

(fn `UserConstructionScript`
  (`parent.UserConstructionScript`))