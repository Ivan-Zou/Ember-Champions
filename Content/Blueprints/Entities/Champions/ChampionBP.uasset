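; Champion entity that follows its referenced squad through AI movement.
; BeginFollow stores a distance threshold and starts a FollowPlayer loop that re-runs after a short delay until EndFollow clears the Follow flag.
; Each pass checks horizontal distance to the squad, ignoring height, and issues a move toward it when beyond the threshold, otherwise a move to its own location to hold position.
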(event `self.ReceiveBeginPlay`
  (`parent.ReceiveBeginPlay`))

(event `Begin Follow`
  (params (Threshold :type "Float (double-precision)"))
  ; Follow Logic
  (set `self.DistanceThreshold` Threshold)
  (set `self.Follow` true)
  (`self.Follow Player`))

(event `End Follow`
  ; Follow Logic
  (set `self.Follow` false))

(event `Follow Player`
  (bind _squadref (`self.SquadRef`))
  ; Follow Logic
  (bind _distance (`self.Get Distance`))
  (if (> _distance (`self.DistanceThreshold`))
    (`|AIMoveTo` self (`self.K2_GetActorLocation` _squadref) _squadref
      (:`then`
        _))
    (else
      (`|AIMoveTo` self (`self.K2_GetActorLocation` self) self
        (:`then`
          _))))
  (`KismetSystemLibrary.Delay` 0.1)
  (if (`self.Follow`)
    (`self.Follow Player`)))

(fn `Get Distance`
  (returns (Distance :type "Float (double-precision)"))
  (bind (_returnvalue_x _returnvalue_y) (`KismetMathLibrary.BreakVector` (`self.K2_GetActorLocation` (`self.SquadRef`))))
  (bind (_returnvalue_x_2 _returnvalue_y_2) (`KismetMathLibrary.BreakVector` (`self.K2_GetActorLocation` self)))
  (return (`KismetMathLibrary.VSize` (`KismetMathLibrary.MakeVector` (- _returnvalue_x_2 _returnvalue_x) (- _returnvalue_y_2 _returnvalue_y)))))

(fn `UserConstructionScript`
  (`parent.UserConstructionScript`))