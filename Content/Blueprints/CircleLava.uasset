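; CircleLava is a lava hazard that drains HP from Archer, Knight, Wizard and Brawler characters standing in it.
; Begin and end overlap events cast the other actor and toggle a flag per class.
; While a flag is set, Tick uses a short Delay to throttle repeated fixed HP deductions.
; Damage hits the first actor found by GetAllActorsOfClass for that class, not the stored overlapping actor.
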(event `self.ReceiveTick`
  (params (DeltaSeconds :type "Float (single-precision)"))
  (`|ExecutionSequence`
    (:`then_0`
      (if (`self.isArcherOverlap`)
        (`KismetSystemLibrary.Delay` 0.1)
        (bind _outactors (`GameplayStatics.GetAllActorsOfClass` "/Game/Blueprints/Entities/Champions/ArcherBP.ArcherBP_C"))
        (bind _output (`|GetArrayItem` _outactors))
        (`/Game/Blueprints/Entities/EntityBP.Set Current HP` _output (- (`/Game/Blueprints/Entities/EntityBP.Current HP` _output) 2))))
    (:`then_1`
      (if (`self.isKnightOverlap`)
        (`KismetSystemLibrary.Delay` 0.1)
        (bind _outactors_2 (`GameplayStatics.GetAllActorsOfClass` "/Game/Blueprints/Entities/Champions/KnightBP.KnightBP_C"))
        (bind _output_2 (`|GetArrayItem` _outactors_2))
        (`/Game/Blueprints/Entities/EntityBP.Set Current HP` _output_2 (- (`/Game/Blueprints/Entities/EntityBP.Current HP` _output_2) 2))))
    (:`then_2`
      (if (`self.isWizardOverlap`)
        (`KismetSystemLibrary.Delay` 0.1)
        (bind _outactors_3 (`GameplayStatics.GetAllActorsOfClass` "/Game/Blueprints/Entities/Champions/WizardBP.WizardBP_C"))
        (bind _output_3 (`|GetArrayItem` _outactors_3))
        (`/Game/Blueprints/Entities/EntityBP.Set Current HP` _output_3 (- (`/Game/Blueprints/Entities/EntityBP.Current HP` _output_3) 2))))
    (:`then_3`
      (if (`self.isBrawlerOverlap`)
        (`KismetSystemLibrary.Delay` 0.1)
        (bind _outactors_4 (`GameplayStatics.GetAllActorsOfClass` "/Game/Blueprints/Entities/Champions/BrawlerBP.BrawlerBP_C"))
        (bind _output_4 (`|GetArrayItem` _outactors_4))
        (`/Game/Blueprints/Entities/EntityBP.Set Current HP` _output_4 (- (`/Game/Blueprints/Entities/EntityBP.Current HP` _output_4) 2))))))

(event `self.ReceiveActorBeginOverlap`
  (params (OtherActor :type "Actor Object Reference"))
  (`|ExecutionSequence`
    (:`then_0`
      (bind _asarcher_bp (cast `/Game/Blueprints/Entities/Champions/ArcherBP` OtherActor))
      (if (`KismetSystemLibrary.IsValid` _asarcher_bp)
        (set `self.isArcherOverlap` true)))
    (:`then_1`
      (bind _asknight_bp (cast `/Game/Blueprints/Entities/Champions/KnightBP` OtherActor))
      (if (`KismetSystemLibrary.IsValid` _asknight_bp)
        (set `self.isKnightOverlap` true)))
    (:`then_2`
      (bind _aswizard_bp (cast `/Game/Blueprints/Entities/Champions/WizardBP` OtherActor))
      (if (`KismetSystemLibrary.IsValid` _aswizard_bp)
        (set `self.isWizardOverlap` true)))
    (:`then_3`
      (bind _asbrawler_bp (cast `/Game/Blueprints/Entities/Champions/BrawlerBP` OtherActor))
      (if (`KismetSystemLibrary.IsValid` _asbrawler_bp)
        (set `self.isBrawlerOverlap` true)))))

(event `self.ReceiveActorEndOverlap`
  (params (OtherActor :type "Actor Object Reference"))
  (`|ExecutionSequence`
    (:`then_0`
      (cast `/Game/Blueprints/Entities/Champions/ArcherBP` OtherActor)
      (set `self.isArcherOverlap` false))
    (:`then_1`
      (cast `/Game/Blueprints/Entities/Champions/KnightBP` OtherActor)
      (set `self.isKnightOverlap` false))
    (:`then_2`
      (cast `/Game/Blueprints/Entities/Champions/WizardBP` OtherActor)
      (set `self.isWizardOverlap` false))
    (:`then_3`
      (cast `/Game/Blueprints/Entities/Champions/BrawlerBP` OtherActor)
      (set `self.isBrawlerOverlap` false))))

(fn `UserConstructionScript`)